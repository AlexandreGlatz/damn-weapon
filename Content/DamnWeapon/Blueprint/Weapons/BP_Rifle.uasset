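; BP_Rifle is a rifle weapon Blueprint that fires physical bullets, tracks its ammo and can be thrown.
; Fire decrements the clamped ammo count and, only if rounds remain afterward, spawns a BP_Bullet at BulletSpawn and launches it with a forward impulse scaled by Strength.
; Throw enables collision and physics on the Fusil1 component, then pushes it forward with a fixed impulse.
; Getters expose current and maximum ammo.
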(event `/Game/DamnWeapon/Blueprint/Weapons/BPI_Weapon.Throw`
  (bind _fusil_1 (`self.fusil_1`))
  (`PrimitiveComponent.SetCollisionEnabled` _fusil_1 "QueryAndPhysics")
  (`PrimitiveComponent.SetSimulatePhysics` _fusil_1 true)
  (`PrimitiveComponent.AddImpulse` _fusil_1 (* (`SceneComponent.GetForwardVector` _fusil_1) 30000.0) "None" false))

(event `/Game/DamnWeapon/Blueprint/Weapons/BPI_Weapon.Fire`
  (bind _ammoempty (`self.DecrementAmmos`))
  (if (not _ammoempty)
    (bind _returnvalue (`|SpawnActorFromClass` "/Game/DamnWeapon/Blueprint/Weapons/BP_Bullet.BP_Bullet_C" (`SceneComponent.K2_GetComponentToWorld` (`self.bulletSpawn`)) "Undefined" "MultiplyWithRoot" null null))
    (bind _bullet (`/Game/DamnWeapon/Blueprint/Weapons/BP_Bullet.bullet` _returnvalue))
    (`PrimitiveComponent.AddImpulse` _bullet (* (`SceneComponent.GetForwardVector` _bullet) (`self.strength`)) "None" false)))

(fn `DecrementAmmos`
  (returns (ammoEmpty :type Boolean))
  (bind _result (`/Engine/EditorBlueprintResources/StandardMacros.DecrementInt` (`self.ammos`))
    (:`  `
      (bind _output_get (set `self.ammos` (`KismetMathLibrary.Clamp` _result 0 (`self.maxAmmos`))))
      (return (<= _output_get 0)))))

(fn `GetAmmos`
  (returns (ammos :type Integer))
  (return (`self.ammos`)))

(fn `GetMaxAmmos`
  (returns (maxAmmos :type Integer))
  (return (`self.maxAmmos`)))

(fn `UserConstructionScript`)
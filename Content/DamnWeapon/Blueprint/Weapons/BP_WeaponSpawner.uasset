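; BP_WeaponSpawner is a pickup actor that periodically spawns a weapon and refills the player's weapons when they touch it.
; A timer started on BeginPlay spawns a BP_Rifle at the WeaponSpawn transform after SpawnTime, following a switch on WeaponType.
; While a weapon is present, sphere overlap by BP_FPSPlayerCharacter calls RefillWeapons with WeaponType, destroys the spawned actor and restarts the timer.
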(event `self.ReceiveBeginPlay`
  (`self.OnWeaponPickedUp`))

(event `OnWeaponPickedUp`
  (`KismetSystemLibrary.K2_SetTimerDelegate` (delegate `SpawnWeapon`) (`self.spawnTime`)))

(event `SpawnWeapon`
  (switch `/Game/DamnWeapon/Blueprint/Weapons/E_WeaponType` (`self.weaponType`)
    (:`NewEnumerator0`
      (bind _returnvalue (`|SpawnActorFromClass` "/Game/DamnWeapon/Blueprint/Weapons/Rifle/BP_Rifle.BP_Rifle_C" (`SceneComponent.K2_GetComponentToWorld` (`self.weaponSpawn`)) "Undefined" "MultiplyWithRoot" null null))
      (set `self.hasWeapon` true))))

(event `self.Sphere.OnComponentBeginOverlap`
  (params (OverlappedComponent :type "PrimitiveComponent Object Reference") (OtherActor :type "Actor Object Reference") (OtherComp :type "PrimitiveComponent Object Reference") (OtherBodyIndex :type Integer) (bFromSweep :type Boolean) (SweepResult :type "HitResult Structure (by ref)"))
  (if (`self.hasWeapon`)
    (bind _asbp_fpsplayer_character (cast `/Game/DamnWeapon/Blueprint/Player/BP_FPSPlayerCharacter` OtherActor))
    (`/Game/DamnWeapon/Blueprint/Player/BPI_Player.RefillWeapons` _asbp_fpsplayer_character (`self.weaponType`))
    (`self.K2_DestroyActor` (stale `SpawnWeapon` _returnvalue))
    (set `self.hasWeapon` false)
    (`self.OnWeaponPickedUp`)))

(fn `UserConstructionScript`)
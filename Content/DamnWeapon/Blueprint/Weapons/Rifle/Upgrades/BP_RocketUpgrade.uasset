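; Rifle upgrade that makes a thrown rifle change colour and then explode; the explosion here is visual only, with no damage logic.
; On the first throw, it gives the owning BP_Rifle mesh a dynamic material and adds a timeline component to the rifle at runtime.
; A colour curve drives the material for one second, then a Niagara explosion spawns and the rifle is destroyed.
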(event `/Game/DamnWeapon/Blueprint/Weapons/Rifle/Upgrades/BPI_Upgrade.OnThrow`
  (bind _returnvalue (`self.GetOwner`))
  (`/Engine/EditorBlueprintResources/StandardMacros.DoOnce` false
    (:`Completed`
      (`/Engine/EditorBlueprintResources/StandardMacros.IsValid` _returnvalue
        (:`Is Valid`
          (bind _asbp_rifle (cast `/Game/DamnWeapon/Blueprint/Weapons/Rifle/BP_Rifle` _returnvalue))
          (bind _returnvalue_2 (`KismetMaterialLibrary.CreateDynamicMaterialInstance` "/Game/DamnWeapon/Materials/Enemies/M_EnemySkin.M_EnemySkin"))
          (`PrimitiveComponent.SetMaterial` (`/Game/DamnWeapon/Blueprint/Weapons/Rifle/BP_Rifle.rifle` _asbp_rifle) 0 _returnvalue_2)
          (bind _returnvalue_3 (`|AddComponentByClass` _returnvalue "/Script/Engine.TimelineComponent"))
          (`TimelineComponent.SetTimelineFinishedFunc` _returnvalue_3 (delegate `Finished`))
          (`TimelineComponent.AddInterpLinearColor` _returnvalue_3 "/Game/DamnWeapon/Blueprint/Weapons/Rifle/Upgrades/C_ExplosionColorCurve.C_ExplosionColorCurve" (delegate `Update`) "None" "None")
          (`TimelineComponent.SetTimelineLength` _returnvalue_3 1.0)
          (`TimelineComponent.PlayFromStart` _returnvalue_3))))))

(event `Update`
  (params (Output :type "LinearColor Structure"))
  (`MaterialInstanceDynamic.SetVectorParameterValue` (stale `/Game/DamnWeapon/Blueprint/Weapons/Rifle/Upgrades/BPI_Upgrade.OnThrow` _returnvalue_2) "Color" Output))

(event `Finished`
  (`NiagaraFunctionLibrary.SpawnSystemAtLocation` "/Game/DamnWeapon/Particles/NiagaraSystems/NS_Explosion.NS_Explosion" (`Actor.K2_GetActorLocation` (`self.GetOwner`)))
  (`Actor.K2_DestroyActor` (`self.GetOwner`)))
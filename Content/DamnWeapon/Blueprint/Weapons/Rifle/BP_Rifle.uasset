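; BP_Rifle is the player's rifle weapon, which fires limited ammo and can be thrown as a physics projectile.
; Upgrade adds a tag-selected component that supplies the bullet class, particles and throw effect, and Fire launches bullets by impulse.
; Fast throw impacts deal game-mode damage, with knockback and throw effect once per pickup, while Tick keeps the actor on the simulated mesh.
; A timeline animates reloading and clears the player's reloading flag.
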(event `self.ReceiveBeginPlay`
  (bind _gmdamnweapon (`/Game/DamnWeapon/Blueprint/FunctionLibraries/FL_Getter.GetGameModeStatic`))
  (set `self.throwingDamages` (`/Game/DamnWeapon/Blueprint/Player/GM_DamnWeapon.throwingDamages` _gmdamnweapon)))

(event `self.ReceiveTick`
  (params (DeltaSeconds :type "Float (single-precision)"))
  (`self.K2_SetActorLocation` (`SceneComponent.K2_GetComponentLocation` (`self.rifle`))))

(event `/Game/DamnWeapon/Blueprint/Weapons/BPI_Weapon.SetIsOwned`
  (params (isOwned :type Boolean))
  (set `self.isOwned` isOwned))

(event `/Game/DamnWeapon/Blueprint/Weapons/BPI_Weapon.Upgrade`
  (params (tag :type "GameplayTag Structure"))
  (bind _returnvalue (`|AddComponentByClass` (`BlueprintMapLibrary.Map_Find` (`self.upgrades`) tag)))
  (bind _output_get (set `self.BP_RifleUpgrade` _returnvalue))
  (`NiagaraComponent.SetAsset` (`self.upgradeParticles`) (`/Game/DamnWeapon/Blueprint/Weapons/Rifle/Upgrades/BP_RifleUpgrade.particles` _output_get) true))

(event `/Game/DamnWeapon/Blueprint/Weapons/BPI_Weapon.Throw`
  (params (thrower :type "Actor Object Reference"))
  (bind _rifle (`self.rifle`))
  (set `self.lastOwner` thrower)
  (`PrimitiveComponent.SetCollisionEnabled` _rifle "QueryAndPhysics")
  (`PrimitiveComponent.SetCollisionResponseToChannel` _rifle "ECC_Pawn" "ECR_Ignore")
  (`SceneComponent.K2_AddLocalRotation` _rifle (struct :`Roll` 15.0) false false)
  (`PrimitiveComponent.SetSimulatePhysics` _rifle true)
  (`PrimitiveComponent.AddImpulseAtLocation` _rifle (* (`SceneComponent.GetForwardVector` _rifle) 15000.0) (`SceneComponent.K2_GetComponentLocation` (`self.Scene`)) "None"))

(event `/Game/DamnWeapon/Blueprint/Weapons/BPI_Weapon.Fire`
  (bind _ammoempty (`self.DecrementAmmos`))
  (if (not _ammoempty)
    (bind _returnvalue (`|SpawnActorFromClass` (`/Game/DamnWeapon/Blueprint/Weapons/Rifle/Upgrades/BP_RifleUpgrade.bulletClass` (`self.BP_RifleUpgrade`)) (`SceneComponent.K2_GetComponentToWorld` (`self.bulletSpawn`)) "Undefined" "MultiplyWithRoot" null null))
    (bind _returnvalue_2 (`self.GetComponentByClass` _returnvalue "/Script/Engine.StaticMeshComponent"))
    (`PrimitiveComponent.AddImpulse` _returnvalue_2 (* (`SceneComponent.GetForwardVector` _returnvalue_2) (`self.strength`)) "None" false)))

(event `/Game/DamnWeapon/Blueprint/Weapons/BPI_Weapon.PlayReloadAnimation`
  (params (startPlacement :type "SceneComponent Object Reference") (endPlacement :type "SceneComponent Object Reference"))
  (bind (_direction _rotation _position) (`Timeline|Timeline` :!via `PlayFromStart`)
    (:`Update`
      (`SceneComponent.K2_SetRelativeLocation` (`self.DefaultSceneRoot`) (`KismetMathLibrary.VLerp` (`SceneComponent.RelativeLocation` startPlacement) (`SceneComponent.RelativeLocation` endPlacement) _position) false false)
      (`SceneComponent.K2_SetRelativeRotation` (`self.rifle`) (`KismetMathLibrary.MakeRotator` 0.0 _rotation) false false))
    (:`Finished`
      (set `/Game/DamnWeapon/Blueprint/Player/BP_FPSPlayerCharacter.isReloading` false (cast `/Game/DamnWeapon/Blueprint/Player/BP_FPSPlayerCharacter` (`GameplayStatics.GetPlayerCharacter` 0) :!pure true)))))

(event `self.rifle.OnComponentHit`
  (params (HitComponent :type "PrimitiveComponent Object Reference") (OtherActor :type "Actor Object Reference") (OtherComp :type "PrimitiveComponent Object Reference") (NormalImpulse :type "Vector Structure") (Hit :type "HitResult Structure (by ref)"))
  (bind _isfast (`self.GetIsFast`))
  (if _isfast
    (message `/Game/DamnWeapon/Blueprint/BPI_Damageable.TakeDamage` OtherActor (`self.throwingDamages`))
    (`/Engine/EditorBlueprintResources/StandardMacros.DoOnce` false :!label _label
      (:`Completed`
        (`/Engine/EditorBlueprintResources/StandardMacros.IsValid` OtherActor
          (:`Is Valid`
            (message `/Game/DamnWeapon/Blueprint/BPI_Damageable.KnockBack` OtherActor (`SceneComponent.GetComponentVelocity` (`self.rifle`)))
            (message `/Game/DamnWeapon/Blueprint/Weapons/Rifle/Upgrades/BPI_Upgrade.MakeThrowEffect` (`self.BP_RifleUpgrade`) (`self.lastOwner`))))))))

(event `/Game/DamnWeapon/Blueprint/Weapons/BPI_Weapon.PickUp`
  (params (location :type "Vector Structure") (rotation :type "Rotator Structure") (parent :type "SceneComponent Object Reference"))
  (bind _rifle (`self.rifle`))
  (`PrimitiveComponent.SetCollisionEnabled` _rifle "NoCollision")
  (`PrimitiveComponent.SetSimulatePhysics` _rifle false)
  (`SceneComponent.K2_SetWorldLocationAndRotation` _rifle location rotation false false)
  (`SceneComponent.K2_AttachToComponent` _rifle parent "None" "KeepWorld" "KeepWorld" "KeepWorld" true)
  (goto _label :!via `Reset`))

(fn `DecrementAmmos`
  (returns (ammoEmpty :type Boolean))
  (bind _result (`/Engine/EditorBlueprintResources/StandardMacros.DecrementInt` (`self.ammos`))
    (:`  `
      (bind _output_get (set `self.ammos` (`KismetMathLibrary.Clamp` _result 0 (`self.maxAmmos`))))
      (return (<= _output_get 0)))))

(fn `GetAmmos`
  (returns (ammos :type Integer))
  (return (`self.ammos`)))

(fn `GetIsFast`
  (returns (isFast :type Boolean))
  (bind (_returnvalue_x _returnvalue_y _returnvalue_z) (`KismetMathLibrary.BreakVector` (`SceneComponent.GetComponentVelocity` (`self.rifle`))))
  (return (and (> (`KismetMathLibrary.Abs` _returnvalue_x) 10.0) (> (`KismetMathLibrary.Abs` _returnvalue_y) 10.0) (> (`KismetMathLibrary.Abs` _returnvalue_z) 10.0))))

(fn `GetIsOwned`
  (returns (isOwned :type Boolean))
  (return (`self.isOwned`)))

(fn `GetMaxAmmos`
  (returns (maxAmmos :type Integer))
  (return (`self.maxAmmos`)))

(fn `UserConstructionScript`)
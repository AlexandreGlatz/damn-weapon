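; BP_Bullet is a rifle bullet actor that deals damage to what it overlaps and then removes itself.
; On BeginPlay it takes its damage value from the static game mode's base bullet damage.
; The Sphere overlap sends TakeDamageMessage to the other actor, then destroys the bullet unless that actor is itself.
; A hit on the Bullet component destroys the actor without dealing damage.
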(event `self.ReceiveBeginPlay`
  (bind _gmdamnweapon (`/Game/DamnWeapon/Blueprint/FunctionLibraries/FL_Getter.GetGameModeStatic`))
  (set `self.damages` (`/Game/DamnWeapon/Blueprint/Player/GM_DamnWeapon.baseBulletDamages` _gmdamnweapon)))

(event `self.Sphere.OnComponentBeginOverlap`
  (params (OverlappedComponent :type "PrimitiveComponent Object Reference") (OtherActor :type "Actor Object Reference") (OtherComp :type "PrimitiveComponent Object Reference") (OtherBodyIndex :type Integer) (bFromSweep :type Boolean) (SweepResult :type "HitResult Structure (by ref)"))
  (message `/Game/DamnWeapon/Blueprint/BPI_Damageable.TakeDamage` OtherActor (`self.damages`))
  (if (not (== OtherActor self))
    (`self.K2_DestroyActor`)))

(event `self.bullet.OnComponentHit`
  (params (HitComponent :type "PrimitiveComponent Object Reference") (OtherActor :type "Actor Object Reference") (OtherComp :type "PrimitiveComponent Object Reference") (NormalImpulse :type "Vector Structure") (Hit :type "HitResult Structure (by ref)"))
  (`self.K2_DestroyActor`))

(fn `UserConstructionScript`)
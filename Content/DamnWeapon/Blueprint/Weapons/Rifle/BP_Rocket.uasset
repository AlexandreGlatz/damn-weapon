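; BP_Rocket is a rocket projectile, filed with the rifle weapons, that explodes and deals area damage.
; When its Sphere overlaps anything other than itself or a BP_Rifle, it unhides the Bullet component and spawns the NS_Explosion effect there.
; It then sends TakeDamage with its Damages value to every actor overlapping the Sphere, unfiltered, and destroys itself.
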(event `self.Sphere.OnComponentBeginOverlap`
  (params (OverlappedComponent :type "PrimitiveComponent Object Reference") (OtherActor :type "Actor Object Reference") (OtherComp :type "PrimitiveComponent Object Reference") (OtherBodyIndex :type Integer) (bFromSweep :type Boolean) (SweepResult :type "HitResult Structure (by ref)"))
  (if (not (or (== OtherActor self) (== (`GameplayStatics.GetObjectClass` OtherActor) "/Game/DamnWeapon/Blueprint/Weapons/Rifle/BP_Rifle.BP_Rifle_C")))
    (`SceneComponent.SetHiddenInGame` (`self.bullet`) false false)
    (`NiagaraFunctionLibrary.SpawnSystemAtLocation` "/Game/DamnWeapon/Particles/NiagaraSystems/NS_Explosion.NS_Explosion" (`SceneComponent.K2_GetComponentLocation` (`self.bullet`)))
    (for _array_element (`PrimitiveComponent.GetOverlappingActors` (`self.Sphere`) null)
      (message `/Game/DamnWeapon/Blueprint/BPI_Damageable.TakeDamage` _array_element (`self.damages`)))
    (`self.K2_DestroyActor`)))

(fn `UserConstructionScript`
  (`parent.UserConstructionScript`))
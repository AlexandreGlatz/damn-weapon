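; BP_BonusSpawner is a pickup point that spawns a bonus for players and respawns it after collection.
; It looks up the actor class in a Bonuses map by BonusType, spawns it at BonusSpawn and marks it owned, either at start or after a timer.
; A sphere overlap by BP_FPSPlayerCharacter passes the BonusType to the character, destroys the spawned actor and restarts the SpawnTime timer.
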(event `self.ReceiveBeginPlay`
  (if (`self.spawnsAtStart`)
    (`self.SpawnBonus`)
    (else
      (`self.OnWeaponPickedUp`))))

(event `OnWeaponPickedUp`
  (`KismetSystemLibrary.K2_SetTimerDelegate` (delegate `SpawnBonus`) (`self.spawnTime`)))

(event `SpawnBonus`
  (bind _returnvalue (`|SpawnActorFromClass` (`BlueprintMapLibrary.Map_Find` (`self.bonuses`) (`self.bonusType`)) (`SceneComponent.K2_GetComponentToWorld` (`self.BonusSpawn`)) "Undefined" "MultiplyWithRoot" null null))
  (message `/Game/DamnWeapon/Blueprint/Weapons/BPI_Weapon.SetIsOwned` _returnvalue true)
  (set `self.hasBonus` true))

(event `self.Sphere.OnComponentBeginOverlap`
  (params (OverlappedComponent :type "PrimitiveComponent Object Reference") (OtherActor :type "Actor Object Reference") (OtherComp :type "PrimitiveComponent Object Reference") (OtherBodyIndex :type Integer) (bFromSweep :type Boolean) (SweepResult :type "HitResult Structure (by ref)"))
  (if (`self.hasBonus`)
    (bind _asbp_fpsplayer_character (cast `/Game/DamnWeapon/Blueprint/Player/BP_FPSPlayerCharacter` OtherActor))
    (`/Game/DamnWeapon/Blueprint/Player/BPI_Player.PickupBonus` _asbp_fpsplayer_character (`self.bonusType`))
    (`self.K2_DestroyActor` (stale `SpawnBonus` _returnvalue))
    (set `self.hasBonus` false)
    (`self.OnWeaponPickedUp`)))

(fn `UserConstructionScript`)
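; Throwing enemy character that picks up weapons and throws them, or strikes in melee, with stats read from game mode data by enemy type.
; Aim, pickup and attack events report through notify messages, presumably to its AI controller, using slerped rotation, sphere traces and AIMoveTo.
; Timelines animate attacks and hit flashes, with a dynamic material tinted by remaining health.
; Knockback briefly enables capsule physics, and death throws any held weapon before destroying the actor.
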(event `self.ReceiveBeginPlay`
  (`|ExecutionSequence`
    (:`then_0`
      (bind _gmdamnweapon (`/Game/DamnWeapon/Blueprint/FunctionLibraries/FL_Getter.GetGameModeStatic`))
      (bind _value (`BlueprintMapLibrary.Map_Find` (`/Game/DamnWeapon/Blueprint/Player/GM_DamnWeapon.enemiesInformations` _gmdamnweapon) "NewEnumerator1"))
      (bind _output_get (set `self.health` (`/Game/DamnWeapon/Blueprint/Enemies/DA_EnemyInfo.health` _value)))
      (set `self.maxHealth` _output_get)
      (set `self.meleeDamages` (`/Game/DamnWeapon/Blueprint/Enemies/DA_EnemyInfo.damages` _value))
      (set `CharacterMovementComponent.MaxWalkSpeed` (`/Game/DamnWeapon/Blueprint/Enemies/DA_EnemyInfo.speed` _value) (`self.CharacterMovement`)))
    (:`then_1`
      (`/Game/DamnWeapon/Blueprint/Enemies/AI/AIC_Enemies.SetType` (cast `/Game/DamnWeapon/Blueprint/Enemies/AI/AIC_Enemies` (`self.GetController`) :!pure true) "NewEnumerator1"))
    (:`then_2`
      (bind _returnvalue (`KismetMaterialLibrary.CreateDynamicMaterialInstance` "/Game/DamnWeapon/Materials/Enemies/M_EnemySkin.M_EnemySkin"))
      (bind _output_get_2 (set `self.material` _returnvalue))
      (`PrimitiveComponent.SetMaterial` (`self.body`) 0 _output_get_2)
      (`PrimitiveComponent.SetMaterial` (`self.nose`) 0 _output_get_2)
      (`MaterialInstanceDynamic.SetVectorParameterValue` _output_get_2 "Color" (struct :`R` 1.0 :`G` 1.0 :`B` 1.0 :`A` 1.0)))))

(event `/Game/DamnWeapon/Blueprint/BPI_Attacker.Aim`
  (params (targetToAim :type "Actor Object Reference"))
  (bind _returnvalue (`self.K2_GetActorLocation`))
  (bind _returnvalue_2 (`SceneComponent.GetForwardVector` (`self.Scene`)))
  ; AIm
  (`/Game/DamnWeapon/Blueprint/BPI_Attacker.RotateToTarget` targetToAim)
  (bind _outhits (`KismetSystemLibrary.SphereTraceMultiForObjects` (+ (* _returnvalue_2 100.0) _returnvalue) (+ _returnvalue (* _returnvalue_2 10000.0)) 10.0 (`|MakeArray` "ObjectTypeQuery1" "ObjectTypeQuery2" "ObjectTypeQuery3" :!type "EObjectTypeQuery Enum")))
  (if (> (`KismetArrayLibrary.Array_Length` _outhits) 0)
    (if (== (`.HitActor` (`GameplayStatics.BreakHitResult` (`|GetArrayItem` _outhits))) targetToAim)
      (message `/Game/DamnWeapon/Blueprint/BPI_Event.Notify` (`self.BP_InLine`)))))

(event `/Game/DamnWeapon/Blueprint/BPI_Attacker.PickupWeapon`
  (params (weapon :type "Actor Object Reference"))
  (bind _weaponplacement (`self.weaponPlacement`))
  (message `/Game/DamnWeapon/Blueprint/BPI_Attacker.RotateToTarget` self weapon)
  (`|AIMoveTo` self (0.0 0.0 0.0) weapon 50.0
    (:`OnSuccess`
      (message `/Game/DamnWeapon/Blueprint/Weapons/BPI_Weapon.PickUp` weapon (`SceneComponent.K2_GetComponentLocation` _weaponplacement) (`SceneComponent.K2_GetComponentRotation` _weaponplacement) (`self.Scene`))
      (message `/Game/DamnWeapon/Blueprint/Weapons/BPI_Weapon.SetIsOwned` weapon true)
      (set `self.currentWeapon` weapon)
      (set `self.hasWeapon` true)
      (message `/Game/DamnWeapon/Blueprint/BPI_Event.Notify` (`self.BP_WeaponPickedUp`)))))

(event `/Game/DamnWeapon/Blueprint/BPI_Attacker.RotateToTarget`
  (params (targetToAim :type "Actor Object Reference"))
  (bind _scene (`self.Scene`))
  (`SceneComponent.K2_SetWorldRotation` (`self.Scene`) (`KismetMathLibrary.Quat_Rotator` (`KismetMathLibrary.Quat_Slerp` (`KismetMathLibrary.Conv_RotatorToQuaternion` (`SceneComponent.K2_GetComponentRotation` _scene)) (`KismetMathLibrary.Conv_RotatorToQuaternion` (`KismetMathLibrary.FindLookAtRotation` (`SceneComponent.K2_GetComponentLocation` _scene) (`self.K2_GetActorLocation` targetToAim))) (* (`GameplayStatics.GetWorldDeltaSeconds`) 10.0))) false false))

(event `/Game/DamnWeapon/Blueprint/BPI_Attacker.MeleeAttack`
  (bind _returnvalue (`self.K2_GetActorLocation`))
  (bind _scene (`self.Scene`))
  (bind (_relativerotation_roll _relativerotation_pitch _relativerotation_yaw) (`KismetMathLibrary.BreakRotator` (`SceneComponent.RelativeRotation` _scene)))
  (bind (_direction _rotation) (`Timeline|AttackAnimation` :!via `PlayFromStart`)
    (:`Update`
      (`SceneComponent.K2_SetRelativeRotation` _scene (`KismetMathLibrary.MakeRotator` _relativerotation_roll _rotation _relativerotation_yaw) false false))
    (:`Finished`
      (message `/Game/DamnWeapon/Blueprint/BPI_Event.Notify` (`self.BP_AttackEndedEvent`))
      (bind _outhit (`KismetSystemLibrary.LineTraceSingleForObjects` _returnvalue (+ _returnvalue (* (`SceneComponent.GetForwardVector` (`self.Scene`)) 200.0)) (`|MakeArray` "ObjectTypeQuery1" "ObjectTypeQuery2" "ObjectTypeQuery3" :!type "EObjectTypeQuery Enum")))
      (message `/Game/DamnWeapon/Blueprint/BPI_Damageable.TakeDamage` (`.HitActor` (`GameplayStatics.BreakHitResult` _outhit)) (`self.meleeDamages`)))))

(event `/Game/DamnWeapon/Blueprint/BPI_Attacker.RangeAttack`
  (bind _currentweapon (`self.currentWeapon`))
  (message `/Game/DamnWeapon/Blueprint/Weapons/BPI_Weapon.Throw` _currentweapon self)
  (message `/Game/DamnWeapon/Blueprint/Weapons/BPI_Weapon.SetIsOwned` _currentweapon false)
  (set `self.hasWeapon` false)
  (set `self.currentWeapon` null))

(event `/Game/DamnWeapon/Blueprint/BPI_Damageable.TakeDamage`
  (params (damage :type Integer))
  (`self.TakeDamageAnim`)
  (bind _output_get (set `self.health` (- (`self.health`) damage)))
  (if (<= _output_get 0)
    (`/Game/DamnWeapon/Blueprint/BPI_Damageable.Die`)))

(event `TakeDamageAnim`
  (bind _scene (`self.Scene`))
  (bind _material (`self.material`))
  (bind (_relativerotation_roll _relativerotation_pitch _relativerotation_yaw) (`KismetMathLibrary.BreakRotator` (`SceneComponent.RelativeRotation` _scene)))
  (bind _returnvalue (`MaterialInstanceDynamic.K2_GetVectorParameterValue` _material "Color"))
  (set `self.startColor` _returnvalue)
  (bind (_direction _coloralphalerp _rotation) (`Timeline|TakeDamageAnimation` :!via `PlayFromStart`)
    (:`Update`
      (`MaterialInstanceDynamic.SetVectorParameterValue` _material "Color" (`KismetMathLibrary.LinearColorLerp` (`self.startColor`) (struct :`R` 50.0 :`A` 1.0) _coloralphalerp))
      (`SceneComponent.K2_SetRelativeRotation` _scene (`KismetMathLibrary.MakeRotator` _relativerotation_roll _rotation _relativerotation_yaw) false false))
    (:`Finished`
      (`MaterialInstanceDynamic.SetVectorParameterValue` (`self.material`) "Color" (make `LinearColor` (/ (`KismetMathLibrary.Conv_IntToDouble` (`self.health`)) (`KismetMathLibrary.Conv_IntToDouble` (`self.maxHealth`))) 0.0 0.0 1.0)))))

(event `/Game/DamnWeapon/Blueprint/BPI_Damageable.KnockBack`
  (params (direction :type "Vector Structure"))
  (bind _capsulecomponent (`self.CapsuleComponent`))
  (set `self.lastKnockback` direction)
  (`PrimitiveComponent.SetSimulatePhysics` _capsulecomponent true)
  (`PrimitiveComponent.AddImpulse` _capsulecomponent (* direction (100.0 100.0 1.5)) "None" false)
  (`KismetSystemLibrary.Delay` 0.2)
  (`PrimitiveComponent.SetSimulatePhysics` _capsulecomponent false))

(event `/Game/DamnWeapon/Blueprint/BPI_Damageable.Die`
  (bind _currentweapon (`self.currentWeapon`))
  (`|ExecutionSequence`
    (:`then_0`
      (`/Engine/EditorBlueprintResources/StandardMacros.IsValid` _currentweapon
        (:`Is Valid`
          (message `/Game/DamnWeapon/Blueprint/Weapons/BPI_Weapon.Throw` _currentweapon null))))
    (:`then_1`
      (`self.K2_DestroyActor`))))

(fn `GetHasWeapon`
  (returns (hasWeapon :type Boolean))
  (return (`self.hasWeapon`)))

(fn `testasync`)

(fn `UserConstructionScript`)
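; Enemy character that constantly turns to face the player and attacks by throwing the weapon it carries.
; Tick smooths rotation toward the player with a frame-time-scaled quaternion slerp.
; PickupWeapon attaches and claims a weapon via messages; Aim sphere-traces forward and triggers RangeAttack, which throws and releases it, if the target is the first hit.
; TakeDamage only subtracts Health, MeleeAttack is an empty stub, and GetHasWeapon exposes the armed state.
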(event `self.ReceiveTick`
  (params (DeltaSeconds :type "Float (single-precision)"))
  (`self.RotateToTarget` (`GameplayStatics.GetPlayerCharacter` 0)))

(event `/Game/DamnWeapon/Blueprint/BPI_Damageable.TakeDamage`
  (params (damage :type Integer))
  (set `self.health` (- (`self.health`) damage)))

(event `/Game/DamnWeapon/Blueprint/BPI_Attacker.PickupWeapon`
  (params (weapon :type "Actor Object Reference"))
  (bind _weaponplacement (`self.weaponPlacement`))
  (message `/Game/DamnWeapon/Blueprint/Weapons/BPI_Weapon.PickUp` weapon (`SceneComponent.K2_GetComponentLocation` _weaponplacement) (`SceneComponent.K2_GetComponentRotation` _weaponplacement) (`self.CapsuleComponent`))
  (message `/Game/DamnWeapon/Blueprint/Weapons/BPI_Weapon.SetIsOwned` weapon true)
  (set `self.currentWeapon` weapon)
  (set `self.hasWeapon` true))

(event `/Game/DamnWeapon/Blueprint/BPI_Attacker.RangeAttack`
  (bind _currentweapon (`self.currentWeapon`))
  (message `/Game/DamnWeapon/Blueprint/Weapons/BPI_Weapon.SetIsOwned` _currentweapon false)
  (message `/Game/DamnWeapon/Blueprint/Weapons/BPI_Weapon.Throw` _currentweapon)
  (set `self.hasWeapon` false)
  (set `self.currentWeapon` null))

(event `/Game/DamnWeapon/Blueprint/BPI_Attacker.MeleeAttack`)

(event `/Game/DamnWeapon/Blueprint/BPI_Attacker.Aim`
  (params (targetToAim :type "Actor Object Reference"))
  (bind _returnvalue (`self.K2_GetActorLocation`))
  (bind _outhits (`KismetSystemLibrary.SphereTraceMultiForObjects` (+ (* (`self.GetActorForwardVector`) 100.0) _returnvalue) (+ _returnvalue (* (`self.GetActorForwardVector`) 10000.0)) 10.0 (`|MakeArray` "ObjectTypeQuery1" "ObjectTypeQuery2" "ObjectTypeQuery3" :!type "EObjectTypeQuery Enum")))
  (if (> (`KismetArrayLibrary.Array_Length` _outhits) 0)
    (if (== (`.HitActor` (`GameplayStatics.BreakHitResult` (`|GetArrayItem` _outhits))) targetToAim)
      (`/Game/DamnWeapon/Blueprint/BPI_Attacker.RangeAttack`))))

(fn `GetHasWeapon`
  (returns (hasWeapon :type Boolean))
  (return (`self.hasWeapon`)))

(fn `RotateToTarget`
  (params (`target to aim` :type "Actor Object Reference"))
  (`self.K2_SetActorRotation` (`KismetMathLibrary.Quat_Rotator` (`KismetMathLibrary.Quat_Slerp` (`KismetMathLibrary.Conv_RotatorToQuaternion` (`self.K2_GetActorRotation`)) (`KismetMathLibrary.Conv_RotatorToQuaternion` (`KismetMathLibrary.FindLookAtRotation` (`self.K2_GetActorLocation`) (`self.K2_GetActorLocation` `target to aim`))) (* (`GameplayStatics.GetWorldDeltaSeconds`) 5.0)))))

(fn `UserConstructionScript`)
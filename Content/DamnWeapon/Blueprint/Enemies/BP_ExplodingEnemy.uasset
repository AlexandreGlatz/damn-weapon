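; BP_ExplodingEnemy is a weaponless suicide enemy that explodes when its health runs out or when told to melee attack.
; It sets its type on the enemy AI controller at start and slowly spins its sphere each tick.
; Death plays a timeline that scales the capsule, then knocks back and damages actors overlapping the explosion collision before destroying itself.
; Incoming knockback briefly enables capsule physics for an impulse.
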(event `self.ReceiveBeginPlay`
  (`/Game/DamnWeapon/Blueprint/Enemies/AI/AIC_Enemies.SetType` (cast `/Game/DamnWeapon/Blueprint/Enemies/AI/AIC_Enemies` (`self.GetController`) :!pure true) "NewEnumerator0"))

(event `/Game/DamnWeapon/Blueprint/BPI_Attacker.RotateToTarget`
  (params (targetToAim :type "Vector Structure")))

(event `self.ReceiveTick`
  (params (DeltaSeconds :type "Float (single-precision)"))
  (`SceneComponent.K2_AddRelativeRotation` (`self.Sphere`) (`KismetMathLibrary.MakeRotator` 0.0 (* DeltaSeconds 10.0)) false false))

(event `/Game/DamnWeapon/Blueprint/BPI_Damageable.KnockBack`
  (params (direction :type "Vector Structure"))
  (bind _capsulecomponent (`self.CapsuleComponent`))
  (`PrimitiveComponent.SetSimulatePhysics` _capsulecomponent true)
  (`PrimitiveComponent.AddImpulse` _capsulecomponent (* direction (100.0 100.0 1.5)) "None" false)
  (`KismetSystemLibrary.Delay` 0.2)
  (`PrimitiveComponent.SetSimulatePhysics` _capsulecomponent false))

(event `/Game/DamnWeapon/Blueprint/BPI_Damageable.TakeDamage`
  (params (damage :type Integer))
  (bind _output_get (set `self.health` (- (`self.health`) damage)))
  (if (<= _output_get 0)
    (`/Game/DamnWeapon/Blueprint/BPI_Damageable.Die`)))

(event `/Game/DamnWeapon/Blueprint/BPI_Damageable.Die`
  (bind _explosioncollision (`self.explosionCollision`))
  (`/Engine/EditorBlueprintResources/StandardMacros.DoOnce` false
    (:`Completed`
      (bind (_direction _scale) (`Timeline|Explosion` :!via `PlayFromStart`)
        (:`Update`
          (`SceneComponent.SetWorldScale3D` (`self.CapsuleComponent`) (`KismetMathLibrary.Conv_DoubleToVector` _scale)))
        (:`Finished`
          (`SceneComponent.SetHiddenInGame` (`self.Sphere`) true false)
          (for _array_element (`PrimitiveComponent.GetOverlappingActors` _explosioncollision null)
            (message `/Game/DamnWeapon/Blueprint/BPI_Damageable.KnockBack` _array_element (* (`KismetMathLibrary.GetDirectionUnitVector` (`SceneComponent.K2_GetComponentLocation` _explosioncollision) (`self.K2_GetActorLocation` _array_element)) (2.0 2.0 10000000.0)))
            (message `/Game/DamnWeapon/Blueprint/BPI_Damageable.TakeDamage` _array_element (`self.explosionDamage`)))
          (`self.K2_DestroyActor`))))))

(event `/Game/DamnWeapon/Blueprint/BPI_Attacker.MeleeAttack`
  (`/Game/DamnWeapon/Blueprint/BPI_Damageable.Die`))

(fn `GetHasWeapon`
  (returns (hasWeapon :type Boolean))
  (return false))

(fn `UserConstructionScript`)
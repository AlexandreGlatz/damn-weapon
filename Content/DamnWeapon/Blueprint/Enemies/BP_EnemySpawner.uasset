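; Enemy spawner actor that registers with WavesManager at BeginPlay and spawns AI enemies at its own location for a given wave.
; SpawnEnemies reads that wave's count from EnemiesPerWave, rolling against each EnemyTypes map chance in order to choose an exploder or thrower.
; Helper functions fill EnemiesPerWave from the manager's wave count: Apply pads or trims it, while ApplyRandom and ApplyFromCurve rebuild it within min/max values.
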(event `self.ReceiveBeginPlay`
  (`KismetArrayLibrary.Array_Add` (`/Game/DamnWeapon/Blueprint/Tools/BP_WavesManager.spawners` (`self.WavesManager`)) self))

(event `/Game/DamnWeapon/Blueprint/BPI_Spawner.SpawnEnemies`
  (params (currentWave :type Integer))
  (bind _returnvalue (`self.K2_GetActorLocation`))
  (for _ (range (`|GetArrayItem` (`self.enemiesPerWave`) currentWave))
    (bind (_keypin _valuepin) (`|MapForEach` (`self.enemyTypes`) :!label _label)
      (:`then`
        (if (< (`KismetMathLibrary.RandomIntegerInRange` 1 100) _valuepin)
          (set `self.enemyType` _keypin)
          (goto _label :!via `BreakPin`)))
      (:`CompletedPin`
        (switch `/Game/DamnWeapon/Blueprint/Enemies/E_EnemyType` (`self.enemyType`)
          (:`NewEnumerator0`
            (`AIBlueprintHelperLibrary.SpawnAIFromClass` "/Game/DamnWeapon/Blueprint/Enemies/BP_ExplodingEnemy.BP_ExplodingEnemy_C" null _returnvalue (struct) false null))
          (:`NewEnumerator1`
            (`AIBlueprintHelperLibrary.SpawnAIFromClass` "/Game/DamnWeapon/Blueprint/Enemies/BP_EnemyCharacter.BP_EnemyCharacter_C" null _returnvalue (struct) false null)))))))

(fn `Apply`
  (bind _enemiesperwave (`self.enemiesPerWave`))
  (bind _returnvalue (`KismetArrayLibrary.Array_Length` (`self.enemiesPerWave`)))
  (bind _wavesamount (`/Game/DamnWeapon/Blueprint/Tools/BP_WavesManager.WavesAmount` (`self.WavesManager`)))
  (if (> _wavesamount _returnvalue)
    (for _ (range _returnvalue 1)
      (`KismetArrayLibrary.Array_Add` _enemiesperwave -1))
    (else
      (while (> _returnvalue _wavesamount)
        (`KismetArrayLibrary.Array_Remove` _enemiesperwave _wavesamount)))))

(fn `ApplyFromCurve`
  (bind _enemiesperwave (`self.enemiesPerWave`))
  (bind _returnvalue (- (`/Game/DamnWeapon/Blueprint/Tools/BP_WavesManager.WavesAmount` (`self.WavesManager`)) 1))
  (`KismetArrayLibrary.Array_Clear` _enemiesperwave)
  (for _index (range (`KismetArrayLibrary.Array_Length` _enemiesperwave) (+ _returnvalue 1))
    (`KismetArrayLibrary.Array_Add` (`self.enemiesPerWave`) (`KismetMathLibrary.FTrunc` (`KismetMathLibrary.Lerp` (`KismetMathLibrary.Conv_IntToDouble` (`self.minEnemiesPerWaves`)) (`KismetMathLibrary.Conv_IntToDouble` (`self.maxEnemiesPerWaves`)) (`CurveFloat.GetFloatValue` (`self.Curve`) (/ (`KismetMathLibrary.Conv_IntToDouble` _index) (`KismetMathLibrary.Conv_IntToDouble` _returnvalue))))))))

(fn `ApplyRandom`
  (bind _enemiesperwave (`self.enemiesPerWave`))
  (`KismetArrayLibrary.Array_Clear` _enemiesperwave)
  (for _ (range (`KismetArrayLibrary.Array_Length` _enemiesperwave) (`/Game/DamnWeapon/Blueprint/Tools/BP_WavesManager.WavesAmount` (`self.WavesManager`)))
    (`KismetArrayLibrary.Array_Add` (`self.enemiesPerWave`) (`KismetMathLibrary.RandomIntegerInRange` (`self.minEnemiesPerWaves`) (`self.maxEnemiesPerWaves`)))))

(fn `UserConstructionScript`)
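; Enemy pawn that picks up weapons, aims and throws them at a target, and can also perform a melee swing.
; Exposes action events, presumably driven by its AI controller, with pickup, line-of-sight and melee completion reported back through notify messages.
; Aiming slerps the Scene component toward the target and sphere-traces forward to confirm a clear line.
; Damage destroys it at zero health, while knockback briefly enables capsule physics for an impulse.
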(event `self.ReceiveBeginPlay`
  (`/Game/DamnWeapon/Blueprint/Enemies/AI/AIC_Enemies.SetType` (cast `/Game/DamnWeapon/Blueprint/Enemies/AI/AIC_Enemies` (`self.GetController`) :!pure true) "NewEnumerator1"))

(event `/Game/DamnWeapon/Blueprint/BPI_Attacker.PickupWeapon`
  (params (weapon :type "Actor Object Reference"))
  (bind _weaponplacement (`self.weaponPlacement`))
  (message `/Game/DamnWeapon/Blueprint/BPI_Attacker.RotateToTarget` self (`self.K2_GetActorLocation` weapon))
  (`|AIMoveTo` self (0.0 0.0 0.0) weapon 50.0
    (:`OnSuccess`
      (message `/Game/DamnWeapon/Blueprint/Weapons/BPI_Weapon.PickUp` weapon (`SceneComponent.K2_GetComponentLocation` _weaponplacement) (`SceneComponent.K2_GetComponentRotation` _weaponplacement) (`self.Scene`))
      (message `/Game/DamnWeapon/Blueprint/Weapons/BPI_Weapon.SetIsOwned` weapon true)
      (set `self.currentWeapon` weapon)
      (set `self.hasWeapon` true)
      (message `/Game/DamnWeapon/Blueprint/BPI_Event.Notify` (`self.BP_WeaponPickedUp`)))))

(event `/Game/DamnWeapon/Blueprint/BPI_Attacker.RotateToTarget`
  (params (targetToAim :type "Vector Structure"))
  (bind _scene (`self.Scene`))
  (`SceneComponent.K2_SetWorldRotation` (`self.Scene`) (`KismetMathLibrary.Quat_Rotator` (`KismetMathLibrary.Quat_Slerp` (`KismetMathLibrary.Conv_RotatorToQuaternion` (`SceneComponent.K2_GetComponentRotation` _scene)) (`KismetMathLibrary.Conv_RotatorToQuaternion` (`KismetMathLibrary.FindLookAtRotation` (`SceneComponent.K2_GetComponentLocation` _scene) targetToAim)) (* (`GameplayStatics.GetWorldDeltaSeconds`) 10.0))) false false))

(event `/Game/DamnWeapon/Blueprint/BPI_Attacker.Aim`
  (params (targetToAim :type "Actor Object Reference"))
  (bind _returnvalue (`self.K2_GetActorLocation`))
  (bind _returnvalue_2 (`SceneComponent.GetForwardVector` (`self.Scene`)))
  (`/Game/DamnWeapon/Blueprint/BPI_Attacker.RotateToTarget` (`self.K2_GetActorLocation` targetToAim))
  (bind _outhits (`KismetSystemLibrary.SphereTraceMultiForObjects` :`Start` (+ (* _returnvalue_2 100.0) _returnvalue) :`End` (+ _returnvalue (* _returnvalue_2 10000.0)) :`Radius` 10.0 :`ObjectTypes` (`|MakeArray` "ObjectTypeQuery1" "ObjectTypeQuery2" "ObjectTypeQuery3" :!type "EObjectTypeQuery Enum") :`DrawDebugType` "ForOneFrame"))
  (if (> (`KismetArrayLibrary.Array_Length` _outhits) 0)
    (if (== (`.HitActor` (`GameplayStatics.BreakHitResult` (`|GetArrayItem` _outhits))) targetToAim)
      (message `/Game/DamnWeapon/Blueprint/BPI_Event.Notify` (`self.BP_InLine`)))))

(event `/Game/DamnWeapon/Blueprint/BPI_Attacker.MeleeAttack`
  (bind _scene (`self.Scene`))
  (bind (_relativerotation_roll _relativerotation_pitch _relativerotation_yaw) (`KismetMathLibrary.BreakRotator` (`SceneComponent.RelativeRotation` _scene)))
  (bind (_direction _rotation) (`Timeline|AttackAnimation` :!via `PlayFromStart`)
    (:`Update`
      (`SceneComponent.K2_SetRelativeRotation` _scene (`KismetMathLibrary.MakeRotator` _relativerotation_roll _rotation _relativerotation_yaw) false false))
    (:`Finished`
      (message `/Game/DamnWeapon/Blueprint/BPI_Event.Notify` (`self.BP_AttackEndedEvent`)))))

(event `/Game/DamnWeapon/Blueprint/BPI_Attacker.RangeAttack`
  (bind _currentweapon (`self.currentWeapon`))
  (message `/Game/DamnWeapon/Blueprint/Weapons/BPI_Weapon.Throw` _currentweapon)
  (message `/Game/DamnWeapon/Blueprint/Weapons/BPI_Weapon.SetIsOwned` _currentweapon false)
  (set `self.hasWeapon` false)
  (set `self.currentWeapon` null))

(event `/Game/DamnWeapon/Blueprint/BPI_Damageable.TakeDamage`
  (params (damage :type Integer))
  (bind _output_get (set `self.health` (- (`self.health`) damage)))
  (if (<= _output_get 0)
    (`/Game/DamnWeapon/Blueprint/BPI_Damageable.Die`)))

(event `/Game/DamnWeapon/Blueprint/BPI_Damageable.KnockBack`
  (params (direction :type "Vector Structure"))
  (bind _capsulecomponent (`self.CapsuleComponent`))
  (set `self.lastKnockback` direction)
  (`PrimitiveComponent.SetSimulatePhysics` _capsulecomponent true)
  (`PrimitiveComponent.AddImpulse` _capsulecomponent (* direction (100.0 100.0 1.5)) "None" false)
  (`KismetSystemLibrary.Delay` 0.2)
  (`PrimitiveComponent.SetSimulatePhysics` _capsulecomponent false))

(event `/Game/DamnWeapon/Blueprint/BPI_Damageable.Die`
  (`self.K2_DestroyActor`))

(fn `GetHasWeapon`
  (returns (hasWeapon :type Boolean))
  (return (`self.hasWeapon`)))

(fn `testasync`)

(fn `UserConstructionScript`)